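; Ranged enemy variant that chases the player and casts projectiles, overriding actor overlap to disable inherited melee behavior.
; While the player is in view and it is not attacking, it uses AI MoveTo, then attacks if a visibility trace finds no blocking hit.
; The attack stops movement, plays a casting montage and immediately spawns a projectile at the actor's transform, with delays timing the cast and cooldown.
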(event `CreateProjectile`
  (`|SpawnActorFromClass` "/Game/Characters/Enemies/BP_Enemy_Projectile.BP_Enemy_Projectile_C" (`self.GetTransform`) "Undefined" "OverrideRootScale" null null))

(event `self.AttemptAttack`
  ;[1 1 1] Ranged attack event
  (if (`self.CanAttack`)
    (bind _returnvalue (`self.PlayAnimMontage` "/Game/ThirdPerson/Montage/CastingMontage.CastingMontage"))
    (`MovementComponent.StopMovementImmediately` (`self.CharacterMovement`))
    (set `self.CanAttack` false)
    (set `self.Attacking` true)
    (`self.CreateProjectile`)
    (`KismetSystemLibrary.Delay` _returnvalue)
    (set `self.Attacking` false)
    (`self.StopAnimMontage` "/Game/ThirdPerson/Montage/CastingMontage.CastingMontage")
    (`KismetSystemLibrary.Delay` (- (`self.AttackCooldown`) _returnvalue))
    (set `self.CanAttack` true)))

(event `self.ChasePlayer`
  ;[1 1 1] Ranged chase event
  (if (`self.PlayerInView`)
    (if (not (`self.Attacking`))
      (`|AIMoveTo` self (0.0 0.0 0.0) (`GameplayStatics.GetPlayerCharacter` 0)
        (:`then`
          (bind _outhit (`KismetSystemLibrary.LineTraceSingle` (`self.K2_GetActorLocation`) (`self.K2_GetActorLocation` (`GameplayStatics.GetPlayerPawn` 0)) "TraceTypeQuery1"))
          (if (not (`GameplayStatics.BreakHitResult` _outhit))
            (`self.AttemptAttack`)))))))

(event `self.ReceiveActorBeginOverlap`
  (params (OtherActor :type "Actor Object Reference"))
  ;[1 1 1] override actor overlap to disable melee events
)

(fn `UserConstructionScript`
  (`parent.UserConstructionScript`))