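; Warrock enemy Blueprint that overrides AttemptAttack to prioritize a jump attack whenever its cooldown is ready, otherwise using a fast melee.
; Each attack plays a montage and locks further attacks until a timed ResetAttack; jumps switch movement to Flying, and the reset restores NavWalking.
; Separate hit-check events damage player 0 by distance, with melee adding a dot-product front check and jump damage ignoring direction.
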(event `CheckAndApplyJumpAttack`
  ;[1 1 1] Jump attack hitbox
  (if true
    (if (< (`self.GetDistanceTo` (`GameplayStatics.GetPlayerPawn` 0)) (`self.JumpAttackRange`))
      (`GameplayStatics.ApplyDamage` (`GameplayStatics.GetPlayerPawn` 0) (`self.JumpAttackDamage`) null self))))

(event `CheckAndApplyMelee`
  ;[1 1 1] Melee hitbox; easier way to check if player is infront and in range
  (if (< (`KismetMathLibrary.Dot_VectorVector` (`SceneComponent.GetForwardVector` (`self.CapsuleComponent`)) (- (`self.K2_GetActorLocation`) (`self.K2_GetActorLocation` (`GameplayStatics.GetPlayerPawn` 0)))) 0.0)
    (if (< (`self.GetDistanceTo` (`GameplayStatics.GetPlayerPawn` 0)) (* (`self.AttackRange`) 1.4))
      (`GameplayStatics.ApplyDamage` (`GameplayStatics.GetPlayerPawn` 0) (`self.Damage`) null self))))

(event `self.AttemptAttack`
  (bind _returnvalue (`AnimationAsset.GetPlayLength` (`self.GetCurrentMontage`)))
  (bind _returnvalue_2 (`AnimationAsset.GetPlayLength` (`self.GetCurrentMontage`)))
  ;[1 1 1] Override Attack; always do jumping attack on cooldown, use melees otherwise
  (if (`self.CanAttack`)
    (if (>= (`KismetSystemLibrary.GetGameTimeInSeconds`) (`self.JumpCooldownTimer`))
      (set `self.CanAttack` false)
      (`MovementComponent.StopMovementImmediately` (`self.CharacterMovement`))
      (`self.PlayAnimMontage` "/Game/Characters/Enemies/Warrok/Animations/Warrock_Jump_Attack_Montage.Warrock_Jump_Attack_Montage")
      (`CharacterMovementComponent.SetMovementMode` (`self.CharacterMovement`) "MOVE_Flying" 0)
      (set `self.JumpCooldownTimer` (+ (+ (`KismetSystemLibrary.GetGameTimeInSeconds`) (`self.JumpCooldown`)) _returnvalue_2))
      (`KismetSystemLibrary.K2_SetTimer` null "ResetAttack" _returnvalue_2)
      (elif (>= (`KismetSystemLibrary.GetGameTimeInSeconds`) (`self.AttackCooldownTime`))
        (set `self.CanAttack` false)
        (`self.PlayAnimMontage` "/Game/Characters/Enemies/Warrok/Animations/Montages/Warrock_Attack_Fast_Montage.Warrock_Attack_Fast_Montage")
        (set `self.AttackCooldownTime` (+ (+ (`KismetSystemLibrary.GetGameTimeInSeconds`) (`self.AttackCooldown`)) _returnvalue))
        (`KismetSystemLibrary.K2_SetTimer` null "ResetAttack" _returnvalue)))))

(event `ResetAttack`
  ;[1 1 1] Override Attack; always do jumping attack on cooldown, use melees otherwise
  (set `self.CanAttack` true)
  (`CharacterMovementComponent.SetMovementMode` (`self.CharacterMovement`) "MOVE_NavWalking" 0))

(fn `UserConstructionScript`
  (`parent.UserConstructionScript`))