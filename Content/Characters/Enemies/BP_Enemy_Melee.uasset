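; Melee enemy character that patrols points or idles until it sees the player or takes damage, then chases and attacks.
; Tick runs a boolean decision tree over death, stun, sight and health, driving AIMoveTo, with low-health retreat to the nearest point gated by HasRetreated.
; Montage-timed attacks with cooldown open an overlap damage window that hits the player.
; Damage triggers hit-react stun or death and delayed destruction.
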(event `self.ReceiveBeginPlay`
  (`self.SetSpeed` (`self.WalkSpeed`)))

(event `SetSpeed`
  (params (Speed :type "Float (double-precision)"))
  (bind _output_get (set `self.CurrentSpeed` Speed))
  (set `CharacterMovementComponent.MaxWalkSpeed` _output_get (`self.CharacterMovement`)))

(event `Retreat`
  ;[1 1 1] Retreat to the nearest world retreat point
  (bind _outactors (`GameplayStatics.GetAllActorsOfClass` "/Game/Characters/Enemies/Enemy_Retreat_Point.Enemy_Retreat_Point_C"))
  (`|AIMoveTo` self (0.0 0.0 0.0) (`.ReturnValue` (`GameplayStatics.FindNearestActor` (`self.K2_GetActorLocation`) _outactors))
    (:`OnSuccess`
      (set `self.HasRetreated` true))))

(event `self.ReceiveTick`
  (params (DeltaSeconds :type "Float (single-precision)"))
  ;[1 1 1] Check for constantly needed things. Decision tree based on booleans
  (if (`self.Dead`)
    (`NavMovementComponent.StopActiveMovement` (`self.CharacterMovement`) :!label _label)
    (`CharacterMovementComponent.SetMovementMode` (`self.CharacterMovement`) "MOVE_Walking" 0)
    (elif (`self.Stunned`)
      (goto _label)
      (else
        ;;[1 1 1] Rotation lock so we don't have weird things happen, and we shouldnt have x/y rotations anyways
        (`self.K2_SetActorRotation` (`KismetMathLibrary.MakeRotator` 0.0 0.0 (.yaw (`self.K2_GetActorRotation`))))
        (if (`self.PlayerInView`)
          ;;[1 1 1] Unit is not stunned or dead, unit is in combat
          (`self.SetSpeed` (`self.RunSpeed`))
          (if (<= (`self.CurrentHealth`) (`self.RetreatHealth`))
            (if (`self.HasRetreated`)
              (`self.Retreat`)
              (else
                (if (not (`self.Attacking`)) :!label _label_2
                  (`self.ChasePlayer`))))
            (else
              (goto _label_2)))
          (else
            ;;[1 1 1] Unit is not stunned or dead, unit is not in combat
            (`self.SetSpeed` (`self.WalkSpeed`))
            (if (> (`KismetArrayLibrary.Array_Length` (`self.PatrolPoints`)) 0)
              (`self.Patrol`)
              (else
                (`self.IdleNoCombat`)))))))))

(event `IdleNoCombat`
  ;[1 1 1] Idle action for enemy when not in combat if no patrol points
)

(event `Patrol`
  ;[1 1 1] Tells the AI controller to pathfind towards the given patrol points, if we have them
  (if (`self.PlayerInView`)
    _
    (elif (!= (`KismetArrayLibrary.Array_Length` (`self.PatrolPoints`)) 0)
      (`/Engine/EditorBlueprintResources/StandardMacros.DoOnce` false :!label _label_3
        (:`Completed`
          (`|AIMoveTo` self (0.0 0.0 0.0) (`|GetArrayItem` (`self.PatrolPoints`) (`self.CurrentPatrolPoint`))
            (:`OnSuccess`
              (set `self.CurrentPatrolPoint` (mod (+ (`self.CurrentPatrolPoint`) 1) (`KismetArrayLibrary.Array_Length` (`self.PatrolPoints`))))
              (goto _label_3 :!via `Reset`))))))))

(event `AttemptAttack`
  ;[1 1 1] Play attack animation if we are allowed to attack
  (if (`self.CanAttack`)
    (if (>= (`KismetSystemLibrary.GetGameTimeInSeconds`) (`self.AttackCooldownTime`))
      (`self.PlayAnimMontage` (`self.AttackAnim`))
      (set `self.CanAttack` false)
      (set `self.CanDealDamage` true)
      (set `self.Attacking` true)
      (`KismetSystemLibrary.Delay` (`AnimationAsset.GetPlayLength` (`self.GetCurrentMontage`)))
      (set `self.CanAttack` true)
      (set `self.CanDealDamage` false)
      (set `self.Attacking` false)
      (set `self.AttackCooldownTime` (+ (`KismetSystemLibrary.GetGameTimeInSeconds`) (`self.AttackCooldown`))))))

(event `ChasePlayer`
  ;[1 1 1] Tell the AI controller to pathfind towards the player. Check for melee attacks.
  (if (`self.PlayerInView`)
    (`|AIMoveTo` self (0.0 0.0 0.0) (`GameplayStatics.GetPlayerCharacter` 0) (`self.AttackRange`)
      (:`OnSuccess`
        (`self.AttemptAttack`)))))

(event `self.ReceiveAnyDamage`
  (params (Damage :type "Float (single-precision)") (DamageType :type "DamageType Object Reference") (InstigatedBy :type "Controller Object Reference") (DamageCauser :type "Actor Object Reference"))
  ;[1 1 1] Decrease health and call appropriate checks. also sets the enemy to chase player currently
  (set `self.CurrentHealth` (- (`self.CurrentHealth`) Damage))
  (`self.AnimDamage`)
  (set `self.PlayerInView` true)
  (if true
    _))

(event `self.PawnSensing.OnSeePawn`
  (params (Pawn :type "Pawn Object Reference"))
  ;[1 1 1] Seen player; update variables
  (set `self.PlayerInView` true))

(event `AnimDamage`
  ;[1 1 1] Choose the appropriate animation  for damage taken (death / stun). Also handles stun timer
  (`/Engine/EditorBlueprintResources/StandardMacros.DoOnce` false :!label _label_4
    (:`Completed`
      (if (<= (`self.CurrentHealth`) 0.0)
        ;[1 1 1] death
        (`self.PlayAnimMontage` (`self.DeathAnim`) 0.8)
        (set `self.Stunned` true)
        (set `self.Dead` true)
        (`KismetSystemLibrary.Delay` 5.0)
        (`self.K2_DestroyActor`)
        (else
          ;[1 1 1] hit, no death
          (`self.PlayAnimMontage` (`self.HitReactAnim`))
          (set `self.Stunned` true)
          (`KismetSystemLibrary.Delay` (`self.StunDuration`))
          (set `self.Stunned` false)
          (goto _label_4 :!via `Reset`))))))

(event `self.ReceiveActorBeginOverlap`
  (params (OtherActor :type "Actor Object Reference"))
  ;[1 1 1] Enemy Damage Handler (currently just tests collision with player)
  (bind _asbp_third_person_character (cast `/Game/ThirdPerson/Blueprints/BP_ThirdPersonCharacter` OtherActor))
  (if (`self.CanDealDamage`)
    (`GameplayStatics.ApplyDamage` _asbp_third_person_character (`self.Damage`))
    (set `self.CanDealDamage` false)))

(fn `UserConstructionScript`)